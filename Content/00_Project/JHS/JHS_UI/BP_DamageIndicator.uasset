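; BP_DamageIndicator is a short-lived actor that shows a floating damage number through its widget component.
; On BeginPlay it passes the damage value and critical-hit flag to the widget.
; It picks an end point randomly offset along up and right vectors supplied by the player character.
; A timeline lerps the actor from its spawn location to that point, then destroys it.
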(event EventBeginPlay
  (Class|BPIUIDamageIndicator|SetDamage(Message) (UserInterface|GetWidget (Variables|Default|GetDamageWidget)) (Variables|Default|GetIn%20Damage) (Variables|Default|GetIs%20Critical%20Hit))
  (bind _output_get (Variables|Default|SetStartPos (Transformation|GetActorLocation)))
  (bind (_out_upvector _out_rightvector) (Class|BPIPlayer|GetVector(Message) (Game|GetPlayerCharacter 0)))
  (Variables|Default|SetEndPos (+ _output_get (* _out_upvector (Math|Random|RandomFloatinRange 8e+01 1e+02)) (* _out_rightvector (Math|Random|RandomFloatinRange -2e+02 2e+02))))
  (bind _새_트랙_0 (Timeline|타임라인 Play)
    (:Update
      (Transformation|SetActorLocation (Math|Vector|Lerp(Vector) (Variables|Default|GetStartPos) (Variables|Default|GetEndPos) _새_트랙_0) false false))
    (:Finished
      (Actor|DestroyActor))))

(fn ConstructionScript)