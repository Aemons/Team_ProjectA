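; BP_Test_Enemy is a test enemy with a simple health pool that responds to incoming damage.
; BeginPlay fills current health from max health, and AnyDamage subtracts each hit from it.
; After each hit it prints either the remaining health or a death message at zero or below, with no further death handling.
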(event EventBeginPlay
  (Variables|Default|SetCurrentHealth (Variables|Default|GetMaxHealth)))

(event Game|Damage|EventAnyDamage
  (params (Damage :type Float%20%28single-precision%29) (DamageType :type Damage%20Type%20Object%20Reference) (InstigatedBy :type Controller%20Object%20Reference) (DamageCauser :type Actor%20Object%20Reference))
  (bind _output_get (Variables|Default|SetCurrentHealth (- (Variables|Default|GetCurrentHealth) Damage)))
  (if (<= _output_get 0.0)
    (Development|PrintString "Dead")
    (else
      (Development|PrintString (Utilities|String|ToString(Float) _output_get)))))

(fn ConstructionScript)