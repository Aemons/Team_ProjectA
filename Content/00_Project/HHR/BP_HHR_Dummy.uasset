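; Test dummy Blueprint for exercising health bar UI updates.
; Pressing the 1 key lowers CurrentHealth by a fixed step while it is above zero, then broadcasts OnDecreaseHealthBar with the new value.
; A per-second stamina drain is present but disconnected, and the other events only call their parent implementations.
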(event EventBeginPlay
  (|CallParentFunction))

(event Collision|EventActorBeginOverlap
  (params (OtherActor :type Actor%20Object%20Reference))
  (|CallParentFunction OtherActor))

(event EventTick
  (params (DeltaSeconds :type Float%20%28single-precision%29))
  (|CallParentFunction DeltaSeconds))

(event Input|KeyboardEvents|1
  (params (Key :type Key%20Structure :default "None"))
  ;[1 1 1] Test용 UI Health bar update
  (:Pressed
    (if (> (Variables|Default|GetCurrentHealth) 0.0)
      (bind _output_get (Variables|Default|SetCurrentHealth (- (Variables|Default|GetCurrentHealth) 1e+01)))
      (Default|CallOnDecreaseHealthBar _output_get))))

(fn ConstructionScript
  (|CallParentFunction))